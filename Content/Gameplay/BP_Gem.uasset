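; BP_Gem is a gem actor that bobs in place and gives collection feedback when destroyed.
; It caches its spawn location on BeginPlay, then each Tick offsets Z around that point with a sine of game time.
; On Destroyed it spawns the NS_Collect effect at its location and plays a 2D collect sound with randomized pitch.
; The pickup trigger and any reward logic are absent from its graphs.
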(event EventBeginPlay
  (Variables|Default|SetrootInitLoc (Transformation|GetActorLocation)))

(event EventTick
  (params (DeltaSeconds :type Float%20%28single-precision%29))
  (bind _returnvalue (Utilities|Time|GetGameTimeinSeconds))
  (bind _rootinitloc (Variables|Default|GetrootInitLoc))
  (bind _returnvalue_2 (Math|Trig|Sin(Radians) _returnvalue))
  (bind (_x _y _z) (Math|Vector|BreakVector _rootinitloc))
  (Transformation|SetActorLocation (Math|Vector|MakeVector _x _y (+ _z (+ _returnvalue_2 (* _returnvalue_2 5.0)))) false false))

(event EventDestroyed
  (Niagara|SpawnSystematLocation "/Game/FX/NS_Collect.NS_Collect" (Transformation|GetActorLocation))
  (Audio|PlaySound2D "/Game/Audio/SND/SND_Collect.SND_Collect" 1.0 (Math|Random|RandomFloatinRange 0.8 1.2) 0.0 0 0))

(fn ConstructionScript)