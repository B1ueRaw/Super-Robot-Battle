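; BP_Spring is a spring pad that launches a SideScrollerCharacter when it overlaps the actor.
; The launch follows an Arrow component's forward vector at a fixed speed, overriding the character's existing velocity.
; Two timelines restart together on launch, offsetting the cap's height and scaling the coil's pivot relative to values cached at BeginPlay.
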(event Collision|EventActorBeginOverlap
  (params (OtherActor :type Actor%20Object%20Reference))
  (bind _asside_scroller_character (Utilities|Casting|CastToSideScrollerCharacter OtherActor))
  (Character|LaunchCharacter _asside_scroller_character (* (Math|Vector|GetForwardVector (Variables|Default|GetArrow)) 1500) true true)
  (Utilities|FlowControl|Sequence
    (:then_0
      (bind _loczadd (Timeline|CapRaise PlayFromStart)
        (:Update
          (Transformation|SetRelativeLocation (Variables|Default|GetSM_Cap) (+ (Variables|Default|GetcapInitLoc) (Math|Vector|MakeVector 0.0 0.0 _loczadd)) false false))))
    (:then_1
      (bind _scalevmulti (Timeline|SpringStretch PlayFromStart)
        (:Update
          (Transformation|SetRelativeScale3D (Variables|Default|GetPivot_Coil) (* (Variables|Default|GetcoilInitScale3D) _scalevmulti)))))))

(event EventBeginPlay
  (Variables|Default|SetcapInitLoc (Variables|/Script/Engine.SceneComponent|GetRelativeLocation (Variables|Default|GetSM_Cap)))
  (Variables|Default|SetcoilInitScale3D (Variables|/Script/Engine.SceneComponent|GetRelativeScale3D (Variables|Default|GetPivot_Coil))))

(fn ConstructionScript)